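; BP_Boolean is a sliding block that gets carved where it overlaps BP_Wall actors when E is pressed, then drops.
; The construction script builds a tessellated dynamic mesh box from BoxCollision's extents, and BeginPlay slides it along Y with a timeline.
; E stops the slide and, per overlapping wall, uses a Geometry Script boolean to subtract the boxes' axis-aligned intersection from its mesh.
; A second timeline then lowers the block and destroys BoxCollision when finished.
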(event EventBeginPlay
  (bind _returnvalue (Transformation|GetActorLocation))
  (Variables|Default|SetInitialLocation _returnvalue)
  (Variables|Default|SetTargetLocation (+ _returnvalue "0.000000,400.000000,0.000000"))
  (bind _새_트랙_0 (Timeline|타임라인 Play)
    (:Update
      (Transformation|SetActorLocation (Math|Vector|Lerp(Vector) (Variables|Default|GetInitialLocation) (Variables|Default|GetTargetLocation) _새_트랙_0) true false))))

(event Collision|EventActorBeginOverlap
  (params (OtherActor :type Actor%20Object%20Reference)))

(event EventTick
  (params (DeltaSeconds :type Float%20%28single-precision%29)))

(event Input|KeyboardEvents|E
  (params (Key :type Key%20Structure))
  (:Pressed
    (bind _새_트랙_0 (Timeline|타임라인 Stop)
      (:Update
        (Transformation|SetActorLocation (Math|Vector|Lerp(Vector) (Variables|Default|GetInitialLocation) (Variables|Default|GetTargetLocation) _새_트랙_0) true false)))))

(event Input|KeyboardEvents|E
  (params (Key :type Key%20Structure))
  (bind _boxcollision (Variables|Default|GetBoxCollision))
  (bind _returnvalue (Components|Box|GetScaledBoxExtent _boxcollision))
  (bind _returnvalue_2 (Transformation|GetWorldLocation _boxcollision))
  (:Pressed
    (for _array_element (Collision|GetOverlappingActors (Variables|Default|GetBoxCollision) "/Game/BP_Wall.BP_Wall_C" :!class /Script/Engine.PrimitiveComponent)
      (bind _asbp_wall (Utilities|Casting|CastToBP_Wall _array_element))
      (Variables|Default|SetMax1 (+ _returnvalue_2 _returnvalue))
      (Variables|Default|SetMin1 (- _returnvalue_2 _returnvalue))
      (Variables|Default|SetMax2 (+ (Transformation|GetWorldLocation (Variables|/Game/BP_Wall.BP_Wall_C|GetBox _asbp_wall)) (Components|Box|GetScaledBoxExtent (Variables|/Game/BP_Wall.BP_Wall_C|GetBox _asbp_wall))))
      (Variables|Default|SetMin2 (- (Transformation|GetWorldLocation (Variables|/Game/BP_Wall.BP_Wall_C|GetBox _asbp_wall)) (Components|Box|GetScaledBoxExtent (Variables|/Game/BP_Wall.BP_Wall_C|GetBox _asbp_wall))))
      (bind _returnvalue_3 (DynamicMeshComponent|GetDynamicMesh (Variables|DynamicMeshActor|GetDynamicMeshComponent)))
      (bind _returnvalue_4 (DynamicMeshActor|AllocateComputeMesh))
      (bind _returnvalue_5 (Class|GeometryScriptLibraryMeshPrimitiveFunctions|AppendBox :TargetMesh _returnvalue_4 :Transform (Math|Transform|MakeTransform (Math|Vector|MakeVector (.x (Math|Transform|InverseTransformLocation (Transformation|GetWorldTransform (Variables|DynamicMeshActor|GetDynamicMeshComponent)) (/ (Math|Vector|MakeVector (+ (Math|Float|Min(Float) (.x (Variables|Default|GetMax1)) (.x (Variables|Default|GetMax2))) (Math|Float|Max(Float) (.x (Variables|Default|GetMin1)) (.x (Variables|Default|GetMin2)))) (+ (Math|Float|Min(Float) (.y (Variables|Default|GetMax1)) (.y (Variables|Default|GetMax2))) (Math|Float|Max(Float) (.y (Variables|Default|GetMin1)) (.y (Variables|Default|GetMin2)))) (+ (Math|Float|Min(Float) (.z (Variables|Default|GetMax1)) (.z (Variables|Default|GetMax2))) (Math|Float|Max(Float) (.z (Variables|Default|GetMin1)) (.z (Variables|Default|GetMin2))))) 2.0))) (.y (Math|Transform|InverseTransformLocation (Transformation|GetWorldTransform (Variables|DynamicMeshActor|GetDynamicMeshComponent)) (/ (Math|Vector|MakeVector (+ (Math|Float|Min(Float) (.x (Variables|Default|GetMax1)) (.x (Variables|Default|GetMax2))) (Math|Float|Max(Float) (.x (Variables|Default|GetMin1)) (.x (Variables|Default|GetMin2)))) (+ (Math|Float|Min(Float) (.y (Variables|Default|GetMax1)) (.y (Variables|Default|GetMax2))) (Math|Float|Max(Float) (.y (Variables|Default|GetMin1)) (.y (Variables|Default|GetMin2)))) (+ (Math|Float|Min(Float) (.z (Variables|Default|GetMax1)) (.z (Variables|Default|GetMax2))) (Math|Float|Max(Float) (.z (Variables|Default|GetMin1)) (.z (Variables|Default|GetMin2))))) 2.0))) (- (.z (Math|Transform|InverseTransformLocation (Transformation|GetWorldTransform (Variables|DynamicMeshActor|GetDynamicMeshComponent)) (/ (Math|Vector|MakeVector (+ (Math|Float|Min(Float) (.x (Variables|Default|GetMax1)) (.x (Variables|Default|GetMax2))) (Math|Float|Max(Float) (.x (Variables|Default|GetMin1)) (.x (Variables|Default|GetMin2)))) (+ (Math|Float|Min(Float) (.y (Variables|Default|GetMax1)) (.y (Variables|Default|GetMax2))) (Math|Float|Max(Float) (.y (Variables|Default|GetMin1)) (.y (Variables|Default|GetMin2)))) (+ (Math|Float|Min(Float) (.z (Variables|Default|GetMax1)) (.z (Variables|Default|GetMax2))) (Math|Float|Max(Float) (.z (Variables|Default|GetMin1)) (.z (Variables|Default|GetMin2))))) 2.0))) (/ (.z (Math|Vector|MakeVector (- (Math|Float|Min(Float) (.x (Variables|Default|GetMax1)) (.x (Variables|Default|GetMax2))) (Math|Float|Max(Float) (.x (Variables|Default|GetMin1)) (.x (Variables|Default|GetMin2)))) (- (Math|Float|Min(Float) (.y (Variables|Default|GetMax1)) (.y (Variables|Default|GetMax2))) (Math|Float|Max(Float) (.y (Variables|Default|GetMin1)) (.y (Variables|Default|GetMin2)))) (- (Math|Float|Min(Float) (.z (Variables|Default|GetMax1)) (.z (Variables|Default|GetMax2))) (Math|Float|Max(Float) (.z (Variables|Default|GetMin1)) (.z (Variables|Default|GetMin2)))))) 2.0))) "0, 0, 0" "1.000000,1.000000,1.000000") :DimensionX (.x (Math|Vector|MakeVector (- (Math|Float|Min(Float) (.x (Variables|Default|GetMax1)) (.x (Variables|Default|GetMax2))) (Math|Float|Max(Float) (.x (Variables|Default|GetMin1)) (.x (Variables|Default|GetMin2)))) (- (Math|Float|Min(Float) (.y (Variables|Default|GetMax1)) (.y (Variables|Default|GetMax2))) (Math|Float|Max(Float) (.y (Variables|Default|GetMin1)) (.y (Variables|Default|GetMin2)))) (- (Math|Float|Min(Float) (.z (Variables|Default|GetMax1)) (.z (Variables|Default|GetMax2))) (Math|Float|Max(Float) (.z (Variables|Default|GetMin1)) (.z (Variables|Default|GetMin2)))))) :DimensionY (.y (Math|Vector|MakeVector (- (Math|Float|Min(Float) (.x (Variables|Default|GetMax1)) (.x (Variables|Default|GetMax2))) (Math|Float|Max(Float) (.x (Variables|Default|GetMin1)) (.x (Variables|Default|GetMin2)))) (- (Math|Float|Min(Float) (.y (Variables|Default|GetMax1)) (.y (Variables|Default|GetMax2))) (Math|Float|Max(Float) (.y (Variables|Default|GetMin1)) (.y (Variables|Default|GetMin2)))) (- (Math|Float|Min(Float) (.z (Variables|Default|GetMax1)) (.z (Variables|Default|GetMax2))) (Math|Float|Max(Float) (.z (Variables|Default|GetMin1)) (.z (Variables|Default|GetMin2)))))) :DimensionZ (.z (Math|Vector|MakeVector (- (Math|Float|Min(Float) (.x (Variables|Default|GetMax1)) (.x (Variables|Default|GetMax2))) (Math|Float|Max(Float) (.x (Variables|Default|GetMin1)) (.x (Variables|Default|GetMin2)))) (- (Math|Float|Min(Float) (.y (Variables|Default|GetMax1)) (.y (Variables|Default|GetMax2))) (Math|Float|Max(Float) (.y (Variables|Default|GetMin1)) (.y (Variables|Default|GetMin2)))) (- (Math|Float|Min(Float) (.z (Variables|Default|GetMax1)) (.z (Variables|Default|GetMax2))) (Math|Float|Max(Float) (.z (Variables|Default|GetMin1)) (.z (Variables|Default|GetMin2)))))) :Debug 0))
      (GeometryScript|Booleans|ApplyMeshBoolean :TargetMesh _returnvalue_3 :ToolMesh _returnvalue_5 :Operation "Subtract" :Debug 0)
      (DynamicMeshActor|ReleaseAllComputeMeshes)
      (Variables|Default|SetTargetLocation (Transformation|GetActorLocation))
      (bind _새_트랙_0 (Timeline|타임라인_1 Play)
        (:Update
          (Transformation|SetActorLocation (Math|Vector|Lerp(Vector) (Variables|Default|GetTargetLocation) (+ (Variables|Default|GetTargetLocation) "0.000000,0.000000,-280.000000") _새_트랙_0) true false))
        (:Finished
          (Components|DestroyComponent (Variables|Default|GetBoxCollision)))))))

(fn ConstructionScript
  (bind _boxcollision (Variables|Default|GetBoxCollision))
  (bind _returnvalue (Components|Box|GetScaledBoxExtent _boxcollision))
  (bind _returnvalue_2 (DynamicMeshComponent|GetDynamicMesh (Variables|DynamicMeshActor|GetDynamicMeshComponent)))
  (bind _returnvalue_3 (DynamicMesh|Reset _returnvalue_2))
  (bind _returnvalue_4 (Class|GeometryScriptLibraryMeshPrimitiveFunctions|AppendBox :TargetMesh _returnvalue_3 :Transform (Math|Transform|MakeTransform (Math|Vector|MakeVector 0.0 0.0 (* (.z _returnvalue) -1.0)) "0, 0, 0" "1.000000,1.000000,1.000000") :DimensionX (* (.x _returnvalue) 2.0) :DimensionY (* (.y _returnvalue) 2.0) :DimensionZ (* (.z _returnvalue) 2.0) :Debug 0))
  (Class|GeometryScriptLibraryMeshSubdivideFunctions|ApplyPNTessellation :TargetMesh _returnvalue_4 :TessellationLevel 5 :Debug 0)
  (Class|DynamicMeshComponent|EnableComplexasSimpleCollision (Variables|DynamicMeshActor|GetDynamicMeshComponent)))