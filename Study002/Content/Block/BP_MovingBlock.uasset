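; Moving block for a block-stacking game that glides toward a point above the last block until dropped.
; DropItem stops the glide, trims the dynamic mesh to its BP_Wall overlap via boolean intersection, then lowers it with a second timeline.
; Touching a Floor- or Block-tagged actor halts descent and reports arrival.
; If either timeline finishes, the block destroys itself and costs the player an attempt, triggering game over at zero.
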(event OnComponentBeginOverlap(BoxCollision)
  (params (OverlappedComponent :type Primitive%20Component%20Object%20Reference) (OtherActor :type Actor%20Object%20Reference) (OtherComp :type Primitive%20Component%20Object%20Reference) (OtherBodyIndex :type Integer) (bFromSweep :type Boolean) (SweepResult :type Hit%20Result%20Structure%20%28by%20ref%29))
  (bind _targetlocation (Variables|Default|GetTargetLocation))
  ;[1 1 1] 아래로 내려가는 로직
  (if (not (Variables|Default|GetIsOverlapped))
    (if (Actor|ActorHasTag OtherActor "Floor")
      (Default|CallOnBlockArrived (Transformation|GetActorLocation) true)
      (Variables|Default|SetIsOverlapped true)
      (bind _newtrack_0 (Timeline|Timeline_1 Stop)
        (:Update
          (Transformation|SetActorLocation (Math|Vector|Lerp(Vector) (Variables|Default|GetTargetLocation) (Math|Vector|MakeVector (.x _targetlocation) (.y _targetlocation) (+ 0.0 0.0)) _newtrack_0) false false))
        (:Finished
          (Actor|DestroyActor)
          (CallFunction|UpdateWidget)
          (Development|PrintString "블록 아래에서 파괴 ")))
      (elif (Actor|ActorHasTag OtherActor "Block")
        (Default|CallOnBlockArrived (Transformation|GetActorLocation) false)
        (Variables|Default|SetIsOverlapped true)
        (Timeline|Timeline_1 Stop)))))

(event Custom|UpdateWidget
  ;[1 1 1] 남은 시도 횟수
  (bind _asbp_player (Utilities|Casting|CastToBP_Player (Game|Player|GetPlayerPawn 0)))
  (bind _output_get (Variables|/Game/Characters/BP_Player.BP_Player_C|SetRemainingAttempts _asbp_player (- (Variables|/Game/Characters/BP_Player.BP_Player_C|GetRemainingAttempts _asbp_player) 1)))
  ;[1 1 1] 게임오버 위젯
  (if (<= _output_get 0)
    (Variables|/Game/Characters/BP_Player.BP_Player_C|SetIsPlayerWin _asbp_player false)
    (Variables|/Game/Characters/BP_Player.BP_Player_C|SetIsGameOver _asbp_player true)
    (Default|GameOver _asbp_player)))

(event Custom|DropItem
  (bind _relativeforwardvector (Variables|Default|GetRelativeForwardVector))
  (bind _extradistance (Variables|Default|GetExtraDistance))
  (bind _returnvalue (* _relativeforwardvector _extradistance))
  ;[1 1 1] 겹친 영역을 자르는 로직
  (Input|DisableInput 0)
  (for _array_element (Collision|GetOverlappingActors (Variables|Default|GetBoxCollision) "/Game/Block/BP_Wall.BP_Wall_C" :!class /Script/Engine.PrimitiveComponent)
    (bind _asbp_wall (Utilities|Casting|CastToBP_Wall _array_element))
    (bind _returnvalue_2 (Class|DynamicBlockActor|GetOverlappedArea (Variables|/Game/Block/BP_Wall.BP_Wall_C|GetBox _asbp_wall)))
    (bind _returnvalue_3 (DynamicMeshComponent|GetDynamicMesh (Variables|Default|GetDynamicMeshComponent)))
    (GeometryScript|Booleans|ApplyMeshBoolean :TargetMesh _returnvalue_3 :ToolMesh _returnvalue_2 :Operation "Intersection" :Debug 0)
    (DynamicMeshActor|ReleaseAllComputeMeshes)
    ;[1 1 1] 아래로 내려가는 로직
    (Utilities|FlowControl|Sequence
      (:then_0
        ;[1 1 1] 블럭이 타겟을 향해 움직임
        (bind _alpha (Timeline|Timeline Stop)
          (:Update
            (Transformation|SetActorLocation (Math|Vector|Lerp(Vector) (Variables|Default|GetInitialLocation) (Math|Vector|MakeVector (.x _returnvalue) (.y _returnvalue) (.z (Variables|Default|GetTargetLocation))) _alpha) false false))
          (:Finished
            (Actor|DestroyActor :!label _label)
            (CallFunction|UpdateWidget)
            (Development|PrintString "블록 아래에서 파괴 "))))
      (:then_1
        (Variables|Default|SetTargetLocation (Transformation|GetActorLocation))
        (if (not (Variables|Default|GetIsOverlapped))
          (bind _newtrack_0 (Timeline|Timeline_1 Play)
            (:Update
              (Transformation|SetActorLocation (Math|Vector|Lerp(Vector) (Variables|Default|GetTargetLocation) (Math|Vector|MakeVector (.x (Variables|Default|GetTargetLocation)) (.y (Variables|Default|GetTargetLocation)) (+ 0.0 0.0)) _newtrack_0) false false))
            (:Finished
              (goto _label)))))))
  (Utilities|FlowControl|Sequence
    (:then_0
      (Timeline|Timeline Stop))
    (:then_1
      (Variables|Default|SetTargetLocation (Transformation|GetActorLocation))
      (if (not (Variables|Default|GetIsOverlapped))
        (Timeline|Timeline_1 Play)))))

(event EventBeginPlay
  ;[1 1 1] 블럭이 타겟을 향해 움직임
  (Variables|Default|SetInitialLocation (Transformation|GetActorLocation))
  (Variables|Default|SetTargetLocation (+ (Variables|Default|GetLastBlockLocation) (Math|Vector|MakeVector 0.0 0.0 (Math|Random|RandomFloatinRange 5e+02 8e+02))))
  (Variables|Default|SetRelativeForwardVector (Math|Vector|Normalize (- (Variables|Default|GetTargetLocation) (Variables|Default|GetInitialLocation))))
  (Variables|Default|SetRelativeRightVector (Math|Vector|MakeVector (* (.y (Variables|Default|GetRelativeForwardVector)) -1.0) (.x (Variables|Default|GetRelativeForwardVector)) (.z (Variables|Default|GetRelativeForwardVector))))
  (Variables|Default|SetRelativeUpVector (Math|Vector|CrossProduct (Variables|Default|GetRelativeForwardVector) (Variables|Default|GetRelativeRightVector)))
  (Variables|Default|SetFinalLocation (+ (Variables|Default|GetTargetLocation) (* (Variables|Default|GetRelativeForwardVector) (Variables|Default|GetExtraDistance))))
  (bind _alpha (Timeline|Timeline Play)
    (:Update
      (Transformation|SetActorLocation (Math|Vector|Lerp(Vector) (Variables|Default|GetInitialLocation) (Math|Vector|MakeVector (.x (* (Variables|Default|GetRelativeForwardVector) (Variables|Default|GetExtraDistance))) (.y (* (Variables|Default|GetRelativeForwardVector) (Variables|Default|GetExtraDistance))) (.z (Variables|Default|GetTargetLocation))) _alpha) false false))
    (:Finished
      (Actor|DestroyActor)
      (CallFunction|UpdateWidget)
      (Development|PrintString "블록 아래에서 파괴 "))))

(fn ConstructionScript)