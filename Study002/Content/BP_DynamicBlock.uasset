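; BP_DynamicBlock is a sliding block that the E key stops, trims against overlapping BP_Wall actors and drops.
; A timeline moves it along +Y from BeginPlay until E stops it.
; For overlapped walls, a Geometry Script boolean subtracts the overlap area from its dynamic mesh, then a second timeline lowers it and destroys its collision box.
; A return-movement timeline is present but unconnected.
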(event EventBeginPlay
  (bind _returnvalue (Transformation|GetActorLocation))
  ;[1 1 1] 현재 위치 + Fvector(0,400,0)  방향으로 가는 로직
  (Variables|Default|SetInitialLocation _returnvalue)
  (Variables|Default|SetTargetLocation (+ _returnvalue "0.000000,400.000000,0.000000"))
  (bind _새_트랙_0 (Timeline|타임라인 Play)
    (:Update
      (Transformation|SetActorLocation (Math|Vector|Lerp(Vector) (Variables|Default|GetInitialLocation) (Variables|Default|GetTargetLocation) _새_트랙_0) true false))))

(event Collision|EventActorBeginOverlap
  (params (OtherActor :type Actor%20Object%20Reference)))

(event EventTick
  (params (DeltaSeconds :type Float%20%28single-precision%29)))

(event Input|KeyboardEvents|E
  (params (Key :type Key%20Structure :default "None"))
  ;[1 1 1] 현재 위치 + Fvector(0,400,0)  방향으로 가는 로직
  (:Pressed
    (bind _새_트랙_0 (Timeline|타임라인 Stop)
      (:Update
        (Transformation|SetActorLocation (Math|Vector|Lerp(Vector) (Variables|Default|GetInitialLocation) (Variables|Default|GetTargetLocation) _새_트랙_0) true false)))))

(event Input|KeyboardEvents|E
  (params (Key :type Key%20Structure :default "None"))
  ;[1 1 1] 겹친 영역을 자르는 로직
  (:Pressed
    (for _array_element (Collision|GetOverlappingActors (Variables|Default|GetBoxCollision) "/Game/BP_Wall.BP_Wall_C" :!class /Script/Engine.PrimitiveComponent)
      (bind _asbp_wall (Utilities|Casting|CastToBP_Wall _array_element))
      (bind _returnvalue (Class|DynamicBlockActor|GetOverlappedArea (Variables|/Game/BP_Wall.BP_Wall_C|GetBox _asbp_wall)))
      (bind _returnvalue_2 (DynamicMeshComponent|GetDynamicMesh (Variables|Default|GetDynamicMeshComponent)))
      (GeometryScript|Booleans|ApplyMeshBoolean :TargetMesh _returnvalue_2 :ToolMesh _returnvalue :Operation "Subtract" :Debug 0)
      (DynamicMeshActor|ReleaseAllComputeMeshes)
      ;[1 0.1593 0.9455] 움직임과 관련된 부분 - 커브의 움직임을 여기서 확인해보시면 됨.
      (Variables|Default|SetTargetLocation (Transformation|GetActorLocation))
      (bind _새_트랙_0 (Timeline|타임라인_1 Play)
        (:Update
          (Transformation|SetActorLocation (Math|Vector|Lerp(Vector) (Variables|Default|GetTargetLocation) (+ (Variables|Default|GetTargetLocation) "0.000000,0.000000,-280.000000") _새_트랙_0) true false))
        (:Finished
          (Components|DestroyComponent (Variables|Default|GetBoxCollision)))))))

(fn ConstructionScript)