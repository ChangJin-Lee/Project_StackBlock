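; Player pawn for a block-dropping game, handling camera movement, block drops and the game's UI widgets.
; On BeginPlay it stores its starting height, adds the Enhanced Input mapping and shows the in-game widget.
; Camera input yaws the controller and moves the pawn vertically, with IsMovable blocking descent below the starting height.
; The drop action calls DropItem on the referenced moving block, and GameOver shows the game-over widget.
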(event Custom|GameOver
  ;[1 1 1] 게임 종료 위젯
  (bind _returnvalue (UserInterface|CreateWidget "/Game/UI/WBP_GameOver.WBP_GameOver_C"))
  (UserInterface|Viewport|AddtoViewport _returnvalue 0))

(event Input|EnhancedActionEvents|EnhancedInputActionIA_MoveCamera
  (params (ActionValue :type Vector%202D%20Structure) (ElapsedSeconds :type Float%20%28double-precision%29) (TriggeredSeconds :type Float%20%28double-precision%29) (InputAction :type Input%20Action%20Object%20Reference :default "/Game/InputPlayer/Actions/IA_MoveCamera.IA_MoveCamera"))
  (bind _returnvalue (Pawn|GetControlRotation :!class /Script/Engine.Pawn))
  (bind _returnvalue_2 (Math|Vector|GetUpVector (Math|Rotator|MakeRotator 0.0 0.0 (.yaw _returnvalue))))
  ;[1 1 1] 카메라를 상하로 움직이거나 좌우로 회전하는 로직
  (Pawn|Input|AddControllerYawInput (.x ActionValue))
  (bind _return_value (CallFunction|IsMovable (.y ActionValue)))
  (if _return_value
    (Pawn|Input|AddMovementInput (Math|Vector|MakeVector (.x _returnvalue_2) (.y _returnvalue_2) (.z _returnvalue_2)) (.y ActionValue) false)))

(event Input|EnhancedActionEvents|EnhancedInputActionIA_DropBlock
  (params (ActionValue :type Float%20%28double-precision%29) (ElapsedSeconds :type Float%20%28double-precision%29) (TriggeredSeconds :type Float%20%28double-precision%29) (InputAction :type Input%20Action%20Object%20Reference :default "/Game/InputPlayer/Actions/IA_DropBlock.IA_DropBlock"))
  (bind _movingblockref (Variables|Default|GetMovingBlockRef))
  ;[1 1 1] DropBlock
  (Utilities|IsValid _movingblockref
    (:Is%20Valid
      (Default|DropItem _movingblockref))))

(event EventBeginPlay
  ;[1 1 1] Enhanced Input
  (Variables|Default|SetInitialLocation (.z (Transformation|GetActorLocation)))
  (bind _asplayer_controller (Utilities|Casting|CastToPlayerController (Pawn|GetController)))
  (Utilities|IsValid (PlayerController|LocalPlayerSubsystems|GetEnhancedInputLocalPlayerSubsystem _asplayer_controller)
    (:Is%20Valid
      (Input|AddMappingContext (PlayerController|LocalPlayerSubsystems|GetEnhancedInputLocalPlayerSubsystem _asplayer_controller) "/Game/InputPlayer/IMC_Player.IMC_Player" 0 "(bIgnoreAllPressedKeysUntilRelease=True,bForceImmediately=False,bNotifyUserSettings=False)")
      ;[1 1 1] 위젯
      (bind _returnvalue (UserInterface|CreateWidget "/Game/UI/WBP_InGame.WBP_InGame_C"))
      (UserInterface|Viewport|AddtoViewport _returnvalue 0))))

(fn ConstructionScript)

(fn IsMovable
  (params (Direction :type Float%20%28double-precision%29))
  (return (Math|Boolean|NANDBoolean (< Direction 0.0) (< (.z (Transformation|GetActorLocation)) (Variables|Default|GetInitialLocation)))))