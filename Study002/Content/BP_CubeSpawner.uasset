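; Spawner actor that drops new BP_MovingBlock actors into what appears to be a block-stacking game.
; A looping timer spawns each block at a random offset around and above the last block location, handing it that location and the player its reference.
; When a block's arrival event reports a higher position, the spawner moves there; otherwise it prints a loss, destroys the newest block and resets the stored location to the origin.
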(event Custom|SpawnBlock
  (bind _newparam (CallFunction|GetRandomSpawnPosition))
  (bind _output_get (Variables|Default|SetSetSpawnLocation (Math|Vector|MakeVector (.x _newparam) (.y _newparam) (.z _newparam))))
  (bind _returnvalue (Game|SpawnActorfromClass "/Game/BP_MovingBlock.BP_MovingBlock_C" (Math|Conversions|ToTransform(Vector) _output_get) "Undefined" "MultiplyWithRoot" 0 0))
  (bind _asbp_player (Utilities|Casting|CastToBP_Player (Game|Player|GetPlayerPawn 0)))
  (Variables|/Game/BP_Player.BP_Player_C|SetMovingBlockRef _asbp_player _returnvalue)
  (Variables|/Game/BP_MovingBlock.BP_MovingBlock_C|SetLastBlockLocation _returnvalue (Variables|Default|GetLastBlockLocation))
  (EventDispatchers|BindEventtoOnBlockArrived _returnvalue (delegate Custom|UpdateLastBlockLocation)))

(event Custom|UpdateLastBlockLocation
  (params (NewLocation :type Vector))
  (if (> (.z NewLocation) (.z (Variables|Default|GetLastBlockLocation)))
    (bind _output_get (Variables|Default|SetLastBlockLocation (Math|Vector|MakeVector (.x NewLocation) (.y NewLocation) (.z NewLocation))))
    (bind _output_get_2 (Variables|Default|SetSpawnerLocation (Math|Vector|MakeVector (.x _output_get) (.y _output_get) (.z _output_get))))
    (Transformation|SetActorLocation _output_get_2 false false)
    (else
      (Development|PrintString "You Lost Block")
      (Actor|DestroyActor (stale Custom|SpawnBlock _returnvalue))
      (Variables|Default|SetLastBlockLocation "0, 0, 0"))))

(event EventBeginPlay
  (Utilities|Time|SetTimerbyEvent (delegate Custom|SpawnBlock) 3.0 true))

(fn ConstructionScript)

(fn MoveSpawner
  (params (NewLocation :type Vector))
  (Transformation|SetActorLocation (Math|Vector|MakeVector (.x NewLocation) (.y NewLocation) (+ (.z NewLocation) (.z (Transformation|GetActorLocation)))) false false))

(fn GetRandomSpawnPosition
  (bind _lastblocklocation (Variables|Default|GetLastBlockLocation))
  (return (Math|Vector|MakeVector (+ (.x _lastblocklocation) (Math|Float|SelectFloat (Math|Random|RandomFloatinRange -2.5e+03 -1e+03) (Math|Random|RandomFloatinRange 1e+03 2.5e+03) (Math|Random|RandomBool))) (+ (.y _lastblocklocation) (Math|Float|SelectFloat (Math|Random|RandomFloatinRange -2.5e+03 -1e+03) (Math|Random|RandomFloatinRange 1e+03 2.5e+03) (Math|Random|RandomBool))) (+ (.z _lastblocklocation) (Math|Random|RandomFloatinRange 1e+03 1.5e+03)))))