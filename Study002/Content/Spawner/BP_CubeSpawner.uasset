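; Spawner for a block-stacking game that registers with BP_Player and, once started, spawns a BP_MovingBlock on a looping timer until game over.
; Each block appears at a random offset around and above the last stacked location and reports back through OnBlockArrived.
; Higher non-floor landings move the spawner and raise the player's stack count, winning at a target height; other landings update the block's widget and destroy it.
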(event Custom|StartSpawningBlocks
  ;[1 0 0] BP_Player를 C++로 만들어야 전체 로직 리팩가능
  ;;[1 1 1] 블록을 생성하는 로직
  (Utilities|Time|SetTimerbyEvent (delegate Custom|SpawnBlock) 3.0 true))

(event Custom|SpawnBlock
  ;[1 0 0] BP_Player를 C++로 만들어야 전체 로직 리팩가능
  ;;[1 1 1] 블록을 생성하는 로직
  (bind _asbp_player (Utilities|Casting|CastToBP_Player (Game|Player|GetPlayerPawn 0)))
  (if (not (Variables|/Game/Characters/BP_Player.BP_Player_C|GetIsGameOver _asbp_player))
    ;;;[1 1 1] C++로 옮길것.
    (bind _newparam (CallFunction|GetRandomSpawnPosition))
    (bind _output_get (Variables|Default|SetSetSpawnLocation (Math|Vector|MakeVector (.x _newparam) (.y _newparam) (.z _newparam))))
    (bind _returnvalue (Game|SpawnActorfromClass "/Game/Block/BP_MovingBlock.BP_MovingBlock_C" (Math|Conversions|ToTransform(Vector) _output_get) "Undefined" "MultiplyWithRoot" 0 0))
    (bind _asbp_player_2 (Utilities|Casting|CastToBP_Player (Game|Player|GetPlayerPawn 0)))
    (Variables|/Game/Characters/BP_Player.BP_Player_C|SetMovingBlockRef _asbp_player_2 _returnvalue)
    (Variables|/Game/Block/BP_MovingBlock.BP_MovingBlock_C|SetLastBlockLocation _returnvalue (Variables|Default|GetLastBlockLocation))
    (EventDispatchers|BindEventtoOnBlockArrived _returnvalue (delegate Custom|UpdateLastBlockLocation))))

(event Custom|UpdateLastBlockLocation
  (params (NewLocation :type Vector) (IsFloor :type Boolean))
  ;[1 0 0] BP_Player를 C++로 만들어야 전체 로직 리팩가능
  ;;[1 1 1] 블록을 생성하는 로직
  (if IsFloor
    (if (Variables|Default|GetIsFloor)
      (Default|UpdateWidget (stale Custom|SpawnBlock _returnvalue) :!label _label)
      (Actor|DestroyActor (stale Custom|SpawnBlock _returnvalue))
      (else
        (Variables|Default|SetIsFloor true)
        (bind _output_get (Variables|Default|SetLastBlockLocation (Math|Vector|MakeVector (.x NewLocation) (.y NewLocation) (.z NewLocation)) :!label _label_2))
        (bind _output_get_2 (Variables|Default|SetSpawnerLocation (Math|Vector|MakeVector (.x _output_get) (.y _output_get) (.z _output_get))))
        (Transformation|SetActorLocation _output_get_2 false false)
        ;;[1 1 1] 블록의 쌓은 높이
        (bind _asbp_player (Utilities|Casting|CastToBP_Player (Game|Player|GetPlayerPawn 0)))
        (bind _output_get_3 (Variables|/Game/Characters/BP_Player.BP_Player_C|SetStackedHeight _asbp_player (+ (Variables|/Game/Characters/BP_Player.BP_Player_C|GetStackedHeight _asbp_player) 1)))
        (if (>= _output_get_3 5)
          (Variables|/Game/Characters/BP_Player.BP_Player_C|SetIsPlayerWin _asbp_player true)
          (Variables|/Game/Characters/BP_Player.BP_Player_C|SetIsGameOver _asbp_player true)
          (Default|GameOver _asbp_player))))
    (elif (> (.z NewLocation) (.z (Variables|Default|GetLastBlockLocation)))
      (goto _label_2)
      (else
        (goto _label)))))

(event EventBeginPlay
  ;[1 0 0] BP_Player를 C++로 만들어야 전체 로직 리팩가능
  (bind _asbp_player (Utilities|Casting|CastToBP_Player (Game|Player|GetPlayerPawn 0)))
  (Variables|/Game/Characters/BP_Player.BP_Player_C|SetCubeSpawner _asbp_player self))

(fn ConstructionScript)

(fn MoveSpawner
  (params (NewLocation :type Vector))
  (Transformation|SetActorLocation (Math|Vector|MakeVector (.x NewLocation) (.y NewLocation) (+ (.z NewLocation) (.z (Transformation|GetActorLocation)))) false false))

(fn GetRandomSpawnPosition
  (bind _lastblocklocation (Variables|Default|GetLastBlockLocation))
  ;[1 1 1] C++로 옮길것.
  (return (Math|Vector|MakeVector (+ (.x _lastblocklocation) (Math|Float|SelectFloat (Math|Random|RandomFloatinRange -2.5e+03 -1e+03) (Math|Random|RandomFloatinRange 1e+03 2.5e+03) (Math|Random|RandomBool))) (+ (.y _lastblocklocation) (Math|Float|SelectFloat (Math|Random|RandomFloatinRange -2.5e+03 -1e+03) (Math|Random|RandomFloatinRange 1e+03 2.5e+03) (Math|Random|RandomBool))) (+ (.z _lastblocklocation) (Math|Random|RandomFloatinRange 1e+03 1.5e+03)))))